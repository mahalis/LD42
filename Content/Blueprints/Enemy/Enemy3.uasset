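; Enemy3 is an enemy variant in a shooter that attacks by firing homing projectiles at the player pawn.
; On BeginPlay it runs the parent logic, then loads its attack interval, health, maximum speed and point value from the game's shared Tunables.
; Its DoAttack event spawns an Enemy3Projectile, sets the ShootyPawn root as its homing target and prints a debug "pew!".
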(event EventBeginPlay
  (bind _shootygame (Variables|Default|GetShootyGame))
  (bind _tunables (Variables|/Game/Blueprints/ShootyGame.ShootyGame_C|GetTunables _shootygame))
  (|CallParentFunction)
  (Variables|Default|SetAttackInterval (.enemy3shotinterval _tunables))
  (Variables|Default|SetHealth (.enemy3health _tunables))
  (Variables|Default|SetMaximumSpeed (.enemy3maxspeed _tunables))
  (Variables|Default|SetPointValue (.enemy3pointvalue _tunables)))

(event Collision|EventActorBeginOverlap
  (params (OtherActor :type Actor%20Object%20Reference))
  (|CallParentFunction OtherActor) ; This node is disabled and will not be called.\nDrag off pins to build functionality.
)

(event EventTick
  (params (DeltaSeconds :type Float%20%28single-precision%29))
  (|CallParentFunction DeltaSeconds) ; This node is disabled and will not be called.\nDrag off pins to build functionality.
)

(event EventDoAttack
  (Development|PrintString "pew!")
  (bind _projectile (CallFunction|MakeProjectile "/Game/Blueprints/Enemy/Enemy3Projectile.Enemy3Projectile_C"))
  (Variables|/Script/Engine.ProjectileMovementComponent|SetHomingTargetComponent (Variables|/Game/Blueprints/ProjectileBase.ProjectileBase_C|GetProjectileMovement _projectile) (Variables|/Game/Blueprints/Player/ShootyPawn.ShootyPawn_C|GetRoot (Variables|Default|GetShootyPawn))))

(fn ConstructionScript
  (|CallParentFunction))