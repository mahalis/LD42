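; ShootyGame drives mouse aiming for the game, turning the cursor position into a world target for the player's ShootyPawn.
; On BeginPlay it sets Game-and-UI input with a locked, visible mouse and caches the first Cursor actor and the player pawn.
; Each Tick, it traces under the mouse against one object type.
; Hits feed UpdateTarget, which flattens Z to zero, teleports the Cursor there and sets the pawn's TargetLocation.
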(event EventBeginPlay
  (bind _returnvalue (Game|GetPlayerController 0))
  (Utilities|FlowControl|Sequence
    (:then_0
      (Input|EnableInput _returnvalue)
      (Class|WidgetBlueprintLibrary|SetFocustoGameViewport)
      (Input|SetInputModeGameandUI _returnvalue 0 "LockAlways" false))
    (:then_1
      (bind _outactors (Actor|GetAllActorsOfClass "/Game/Blueprints/Cursor.Cursor_C"))
      (Variables|WorldItems|SetCursor (Utilities|Array|Get(acopy) _outactors))
      (bind _asshooty_pawn (Utilities|Casting|CastToShootyPawn (Game|Player|GetPlayerPawn 0)))
      (Variables|WorldItems|SetPlayerPawn _asshooty_pawn))))

(event EventTick
  (params (DeltaSeconds :type Float%20%28single-precision%29))
  (bind _returnvalue (Game|GetPlayerController 0))
  (bind _array (Utilities|Array|MakeArray "ObjectTypeQuery9"))
  (bind (_hitresult _returnvalue_2) (Class|PlayerController|GetHitResultUnderCursorforObjects _returnvalue _array true))
  (if _returnvalue_2
    (CallFunction|UpdateTarget (.Location (Collision|BreakHitResult _hitresult)))))

(fn ConstructionScript)

(fn UpdateTarget
  (params (TargetLocation :type Vector))
  (bind _returnvalue (Math|Vector|MakeVector (.x TargetLocation) (.y TargetLocation) 0.0))
  (Transformation|SetWorldLocation (Variables|/Script/Engine.Actor|GetRootComponent (Variables|WorldItems|GetCursor)) _returnvalue false true)
  (Variables|/Game/Blueprints/Player/ShootyPawn.ShootyPawn_C|SetTargetLocation (Variables|WorldItems|GetPlayerPawn) _returnvalue))