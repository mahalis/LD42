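; PlayerBeam is a player beam actor with a warm-up visual and an active beam visual.
; WarmUp shows the Cube, Begin swaps it for the Cylinder, and End hides the Cylinder.
; DamageStuffInBeam collects EnemyBase actors whose world location, projected on the root's right vector, is under a fixed length; its damage loop is empty.
; BeginPlay caches the ShootyGame game mode.
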(event EventBeginPlay
  (bind _asshooty_game (Utilities|Casting|CastToShootyGame (Game|GetGameMode)))
  (Variables|Default|SetShootyGame _asshooty_game))

(fn ConstructionScript)

(fn DamageStuffinBeam
  (bind _outactors (Actor|GetAllActorsOfClass "/Game/Blueprints/Enemy/EnemyBase.EnemyBase_C"))
  (for _array_element _outactors
    (if (< (Math|Vector|VectorLength (Math|Vector|ProjectVectorontoVector (Transformation|GetActorLocation _array_element) (Math|Vector|GetRightVector (Variables|Default|GetDefaultSceneRoot)))) 5e+01)
      (Utilities|Array|Add (LocalVariables|GetEnemiesInBeam) _array_element)))
  (for _array_element_2 (LocalVariables|GetEnemiesInBeam)
    _))

(fn Begin
  (Rendering|SetVisibility (Variables|Default|GetCylinder) true false)
  (Rendering|SetVisibility (Variables|Default|GetCube) false false))

(fn End
  (Rendering|SetVisibility (Variables|Default|GetCylinder) false false))

(fn WarmUp
  (Rendering|SetVisibility (Variables|Default|GetCube) true false))