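; Base enemy for a top-down shooter that flies into the arena, roams, faces the player and attacks.
; It ignores WorldStatic collision until inside the bounds, then a timer picks destinations with clear lines from the player's obstruction directions, falling back to random points.
; Clamped spring steering drives swept movement with wall bounces.
; Box-trace-gated attacks call an empty DoAttack, and death notifies the game mode while the body keeps drifting.
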(event EventBeginPlay
  (Utilities|FlowControl|Sequence
    (:then_0
      (bind _asshooty_game (Utilities|Casting|CastToShootyGame (Game|GetGameMode)))
      (Variables|References|SetShootyGame _asshooty_game)
      (bind _asshooty_pawn (Utilities|Casting|CastToShootyPawn (Game|Player|GetPlayerPawn 0)))
      (Variables|References|SetShootyPawn _asshooty_pawn))
    (:then_1
      (Collision|SetCollisionResponsetoChannel (Variables|Default|GetBox) "ECC_WorldStatic" "ECR_Ignore")
      (Variables|Attacking|SetNextAttackTime (+ (Utilities|Time|GetGameTimeinSeconds) (Math|Random|RandomFloatinRange 2.0 3.0))))))

(event Collision|EventActorBeginOverlap
  (params (OtherActor :type Actor%20Object%20Reference)))

(event EventTick
  (params (DeltaSeconds :type Float%20%28single-precision%29))
  (Movement|DoMovement)
  (Thinking|CheckWorldEntry)
  (if (Variables|Life|GetIsAlive)
    (Attacking|AttackifPossible)))

(event Collision|EventHit
  (params (MyComp :type Primitive%20Component%20Object%20Reference) (Other :type Actor%20Object%20Reference) (OtherComp :type Primitive%20Component%20Object%20Reference) (bSelfMoved :type Boolean) (HitLocation :type Vector :default "0, 0, 0") (HitNormal :type Vector :default "0, 0, 0") (NormalImpulse :type Vector :default "0, 0, 0") (Hit :type Hit%20Result%20Structure%20%28by%20ref%29))
  (Utilities|Casting|CastToShootyPawn Other
    (:CastFailed
      (Utilities|Casting|CastToProjectileBase Other
        (:then
          (if (Variables|Life|GetIsAlive) ; TODO: impact effects, probably
            _))
        (:CastFailed
          (Movement|Bounce (Math|Vector|MakeVector (.x HitNormal) (.y HitNormal) 0.0) (Variables|Movement|GetWallRestitution)))))))

(fn ConstructionScript)

(fn TakeDamage
  (params (Amount :type Integer) (Location :type Vector) (IncomingVelocity :type Vector))
  (if (Variables|Life|GetIsAlive)
    (Development|PrintString (Utilities|String|BuildString(Integer) "" "oh no, " Amount " damage"))
    (bind _output_get (Variables|Life|SetHealth (Math|Integer|Max(Integer) (- (Variables|Life|GetHealth) Amount))))
    (if (== _output_get 0)
      (Life|Die))))

(fn Die
  (Variables|Life|SetIsAlive false)
  (Collision|SetCollisionObjectType (Variables|Default|GetBox) "ECC_GameTraceChannel4") ; TODO: effects, etc.
  (Utilities|Time|ClearandInvalidateTimerbyHandle (Variables|Thinking|GetWanderTimer))
  (Rendering|Material|SetMaterial (Variables|Default|GetBody) 0 "/Game/Materials/DeadEnemyMaterial.DeadEnemyMaterial")
  (Default|NoteEnemyDeath (Variables|References|GetShootyGame) self))

(fn DoMovement
  (if (Variables|Life|GetIsAlive)
    (Movement|UpdateMoveVelocity))
  (Transformation|AddActorWorldOffset (* (Variables|Movement|GetMoveVelocity) (Utilities|Time|GetWorldDeltaSeconds)) true)
  (if (Variables|Life|GetIsAlive)
    (Movement|DoRotation)))

(fn ChooseRandomDestination
  (bind _shootygame (Variables|References|GetShootyGame))
  (bind _worldhalfsize (Variables|/Game/Blueprints/ShootyGame.ShootyGame_C|GetWorldHalfSize _shootygame))
  (Variables|Movement|SetCurrentDestination (Math|Vector|MakeVector (+ (Math|Random|RandomFloatinRange (* (.x _worldhalfsize) -1.0) (.x _worldhalfsize)) (.z _worldhalfsize)) (Math|Random|RandomFloatinRange (* (.y _worldhalfsize) -1.0) (.y _worldhalfsize)) 0.0)))

(fn FindBestNewDestination
  (bind _shootypawn (Variables|References|GetShootyPawn))
  (bind _array_element (Utilities|Array|ForEachLoopwithBreak (Variables|/Game/Blueprints/Player/ShootyPawn.ShootyPawn_C|GetObstructionDirections _shootypawn) :!label _label)
    (:LoopBody
      (if (> (Math|Vector|VectorLength (Math|Vector|MakeVector (.x _array_element) (.y _array_element) 0.0)) 2e+02) ; is the trace more than a min distance from the player?
        (bind _returnvalue (Collision|LineTraceForObjects (Transformation|GetWorldLocation (Variables|Default|GetRoot)) (+ (Math|Vector|MakeVector (.x _array_element) (.y _array_element) 0.0) (Transformation|GetActorLocation _shootypawn)) (Utilities|Array|MakeArray "ObjectTypeQuery1" "ObjectTypeQuery10") false 0 "None"))
        (if (not _returnvalue) ; is this destination unobstructed both to and from us?
          (Variables|Movement|SetCurrentDestination (+ (Math|Vector|MakeVector (.x _array_element) (.y _array_element) 0.0) (Transformation|GetActorLocation _shootypawn)))
          (LocalVariables|SetFound true)
          (goto _label Break))))
    (:Completed
      (if (not (LocalVariables|GetFound))
        (Thinking|ChooseRandomDestination) ; no good destination; pick a random one
      ))))

(fn Bounce
  (params (Normal :type Vector) (Restitution :type Float%20%28single-precision%29))
  (Variables|Movement|SetMoveVelocity (Math|Vector|GetReflectionVector (Variables|Movement|GetMoveVelocity) (* Normal Restitution))))

(fn UpdateMoveVelocity
  (bind _currentdestination (Variables|Movement|GetCurrentDestination))
  (bind _root (Variables|Default|GetRoot))
  (bind _returnvalue (Transformation|GetWorldLocation _root))
  (bind _returnvalue_2 (- _currentdestination _returnvalue))
  (Variables|Movement|SetMoveVelocity (* (Math|Vector|ClampVectorSize (+ (Variables|Movement|GetMoveVelocity) (* (Math|Vector|ClampVectorSize (* _returnvalue_2 (Variables|Movement|GetDestinationSpringConstant)) 0.0 (Variables|Movement|GetSpringForceLimit)) (Utilities|Time|GetWorldDeltaSeconds))) 0.0 (Variables|Movement|GetMaximumSpeed)) (- 1.0 (* (- 1.0 (Math|Float|Clamp(Float) (/ (Math|Vector|VectorLength _returnvalue_2) 4e+02) 0.4)) (Utilities|Time|GetWorldDeltaSeconds)))))
  (return))

(fn CheckWorldEntry
  (bind _shootygame (Variables|References|GetShootyGame))
  (bind _root (Variables|Default|GetRoot))
  (bind _returnvalue (Transformation|GetWorldLocation _root))
  (bind _worldhalfsize (Variables|/Game/Blueprints/ShootyGame.ShootyGame_C|GetWorldHalfSize _shootygame))
  (if (not (Variables|Thinking|GetHasEnteredWorld))
    (if (and (Math|Float|InRange(Float) (- (.x _returnvalue) (.z _worldhalfsize)) (* (.x _worldhalfsize) -1.0) (.x _worldhalfsize)) (Math|Float|InRange(Float) (.y _returnvalue) (* (.y _worldhalfsize) -1.0) (.y _worldhalfsize)))
      (Collision|SetCollisionResponsetoChannel (Variables|Default|GetBox) "ECC_WorldStatic" "ECR_Block")
      (Variables|Thinking|SetHasEnteredWorld true)
      (Thinking|ChooseRandomDestination)
      (bind _returnvalue_2 (Utilities|Time|SetTimerbyFunctionName 0 "FindBestNewDestination" 4.0 true)) ; TODO: make the time differnt for different enemy types?
      (Variables|Thinking|SetWanderTimer _returnvalue_2))))

(fn DoAttack)

(fn DebugShowDestination
  (Rendering|Debug|DrawDebugLine (Transformation|GetWorldLocation (Variables|Default|GetRoot)) (Variables|Movement|GetCurrentDestination) "(R=0.067292,G=0.875000,B=0.213780,A=1.000000)" 0.0 5.0))

(fn AttackifPossible
  (if (Math|Boolean|ANDBoolean (> (Utilities|Time|GetGameTimeinSeconds) (Variables|Attacking|GetNextAttackTime)) (Variables|Thinking|GetHasEnteredWorld) (Variables|/Game/Blueprints/ShootyGame.ShootyGame_C|GetIsPlaying (Variables|References|GetShootyGame)))
    (bind _returnvalue (Class|KismetSystemLibrary|BoxTraceSingleforObjects (Transformation|GetWorldLocation (Variables|Default|GetRoot)) (Transformation|GetActorLocation (Variables|References|GetShootyPawn)) "8.000000,8.000000,8.000000" "0, 0, 0" (Utilities|Array|MakeArray "ObjectTypeQuery1") true 0 "None" true))
    (if (not _returnvalue) ; if the trace didn't hit anything, we have a clear shot
      (Attacking|DoAttack)
      (Variables|Attacking|SetNextAttackTime (+ (Utilities|Time|GetGameTimeinSeconds) (Variables|Attacking|GetAttackInterval))))))

(fn DoRotation
  (bind _root (Variables|Default|GetRoot))
  (Transformation|SetWorldRotation _root (Math|Conversions|RotationFromXVector (- (Transformation|GetActorLocation (Variables|References|GetShootyPawn)) (Transformation|GetWorldLocation _root))) false false))

(fn MakeProjectile
  (params (Class :type Projectile%20Base%20Class%20Reference))
  (bind _root (Variables|Default|GetRoot))
  (bind _returnvalue (Transformation|GetWorldLocation _root))
  (bind _returnvalue_2 (Game|SpawnActorfromClass Class (Math|Transform|MakeTransform _returnvalue (Math|Rotator|MakeRotator 0.0 0.0 (.yaw (Math|Conversions|RotationFromXVector (- (Transformation|GetActorLocation (Variables|References|GetShootyPawn)) _returnvalue)))) "1,1,1") "AlwaysSpawn" self 0))
  (return _returnvalue_2))