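; Enemy1 is a shooting enemy Blueprint that fires Enemy1Projectile shots.
; On BeginPlay it runs the parent logic, then sets attack interval, health and maximum speed from the shared ShootyGame Tunables.
; Its DoAttack event prints a debug "pew!" and calls MakeProjectile, while the file itself holds no timing or movement logic.
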(event EventBeginPlay
  (bind _shootygame (Variables|Default|GetShootyGame))
  (bind _tunables (Variables|/Game/Blueprints/ShootyGame.ShootyGame_C|GetTunables _shootygame))
  (|CallParentFunction)
  (Variables|Default|SetAttackInterval (.enemy1shotinterval _tunables))
  (Variables|Default|SetHealth (.enemy1health _tunables))
  (Variables|Default|SetMaximumSpeed (.enemy1maxspeed _tunables)))

(event Collision|EventActorBeginOverlap
  (params (OtherActor :type Actor%20Object%20Reference))
  (|CallParentFunction OtherActor) ; This node is disabled and will not be called.\nDrag off pins to build functionality.
)

(event EventTick
  (params (DeltaSeconds :type Float%20%28single-precision%29))
  (|CallParentFunction DeltaSeconds) ; This node is disabled and will not be called.\nDrag off pins to build functionality.
)

(event EventDoAttack
  (Development|PrintString "pew!")
  (CallFunction|MakeProjectile "/Game/Blueprints/Enemy/Enemy1Projectile.Enemy1Projectile_C"))

(fn ConstructionScript
  (|CallParentFunction))