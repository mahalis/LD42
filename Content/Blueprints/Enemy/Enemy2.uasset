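; Enemy2 is a ranged enemy Blueprint that sets its own attack interval and health on BeginPlay after calling the parent.
; Its DoAttack event prints a debug "pew!" and spawns an Enemy2Projectile at its root, owned by itself and yawed toward ShootyPawn.
; After spawning, it writes ProjectileSpeed into the projectile movement's initial and max speed.
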(event EventBeginPlay
  (|CallParentFunction)
  (Variables|Default|SetAttackInterval 2.0)
  (Variables|Default|SetHealth 12))

(event Collision|EventActorBeginOverlap
  (params (OtherActor :type Actor%20Object%20Reference))
  (|CallParentFunction OtherActor) ; This node is disabled and will not be called.\nDrag off pins to build functionality.
)

(event EventTick
  (params (DeltaSeconds :type Float%20%28single-precision%29))
  (|CallParentFunction DeltaSeconds) ; This node is disabled and will not be called.\nDrag off pins to build functionality.
)

(event EventDoAttack
  (bind _root (Variables|Default|GetRoot))
  (bind _projectilespeed (Variables|Default|GetProjectileSpeed))
  (bind _returnvalue (Transformation|GetWorldLocation _root))
  (Development|PrintString "pew!")
  (bind _returnvalue_2 (Game|SpawnActorfromClass "/Game/Blueprints/Enemy/Enemy2Projectile.Enemy2Projectile_C" (Math|Transform|MakeTransform _returnvalue (Math|Rotator|MakeRotator 0.0 0.0 (.yaw (Math|Conversions|RotationFromXVector (- (Transformation|GetActorLocation (Variables|Default|GetShootyPawn)) _returnvalue)))) "1,1,1") "AlwaysSpawn" self 0))
  (Variables|/Script/Engine.ProjectileMovementComponent|SetInitialSpeed (Variables|/Game/Blueprints/ProjectileBase.ProjectileBase_C|GetProjectileMovement _returnvalue_2) _projectilespeed)
  (Variables|/Script/Engine.ProjectileMovementComponent|SetMaxSpeed (Variables|/Game/Blueprints/ProjectileBase.ProjectileBase_C|GetProjectileMovement _returnvalue_2) _projectilespeed))

(fn ConstructionScript
  (|CallParentFunction))